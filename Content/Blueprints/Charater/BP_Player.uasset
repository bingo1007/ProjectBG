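; Player Blueprint that handles movement, camera turning, free look, pose state and item pickups.
; Free look saves the control rotation, unlocks controller yaw and keeps movement aligned to that saved rotation.
; On release, a timeline lerps the control rotation back along the shortest path, then relocks yaw.
; Pickups read DT_ItemInfo by row name, add HP, Speed and Attack, then show the item and stats in the BP_HUD widget.
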(event `self.ReceiveTick`
  (params (DeltaSeconds :type "Float (single-precision)"))
  ; 지터링이라는 문제 발생 고위험 == 캐릭터가 덜덜 떨리는 현상(Jittering)
)

(event `OnFreeLookEnded`
  (bind (_direction _alpha) (`Timeline|Timeline` :!via `PlayFromStart`)
    (:`Update`
      (`Controller.SetControlRotation` (`self.GetController`) (`KismetMathLibrary.RLerp` (`self.EndRotation`) (`self.StartRotation`) _alpha true)))
    (:`Finished`
      (set `self.bUseControllerRotationYaw` true))))

(fn `FreeLook`
  (params (IsPressed :type Boolean))
  (bind _returnvalue (`self.GetControlRotation`))
  (if IsPressed
    (set `self.StartRotation` _returnvalue)
    (set `self.bUseControllerRotationYaw` false)
    (else
      (set `self.EndRotation` _returnvalue)
      (`self.OnFreeLookEnded`))))

(fn `GetMoveRotation`
  (returns (Result :type "Rotator Structure"))
  (return (`KismetMathLibrary.SelectRotator` (`/Game/Blueprints/Util/MathUtils.GetYawOnlyRotation` self) (`self.StartRotation`) (`self.bUseControllerRotationYaw`))))

(fn `InputLookUp`
  (params (YAxis :type "Float (double-precision)"))
  (`self.AddControllerPitchInput` YAxis))

(fn `InputTurn`
  (params (XAxis :type "Float (double-precision)"))
  (`self.AddControllerYawInput` XAxis))

(fn `Move`
  (params (IsForward :type Boolean) (AxisValue :type "Float (double-precision)"))
  (bind _result (`self.GetMoveRotation`))
  ; 이동
  (if IsForward
    (`self.AddMovementInput` (`KismetMathLibrary.GetForwardVector` _result) (`local.AxisValue`))
    (else
      (`self.AddMovementInput` (`KismetMathLibrary.GetRightVector` _result) (`local.AxisValue`)))))

(fn `OnPickUpItem`
  (params (RowName :type Name))
  (locals (ItemInfo :type "/Game/Blueprints/Charater/Test/ST_ItemInfo Structure"))
  ; 로우네임을 기반으로 데이터 테이블에서 정보 가져오기
  ; 찾으면 found, 못찾으면 아래 실행
  (bind _returnvalue (`|GetDataTableRow` "/Game/Blueprints/Charater/Test/DT_ItemInfo.DT_ItemInfo" RowName)
    (:`then`
      (bind _output_get (set `local.ItemInfo` _returnvalue))
      (set `self.HP` (+ (`.HP_10_437A9FEE42469F05E5DD86A4160EC5EB` (break `/Game/Blueprints/Charater/Test/ST_ItemInfo` _output_get)) (`self.HP`)))
      (set `self.Speed` (+ (`.Speed_11_414490944444EC2CD5AADFA481CC5C83` (break `/Game/Blueprints/Charater/Test/ST_ItemInfo` _output_get)) (`self.Speed`)))
      (set `self.Attack` (+ (`.Attack_12_9823DDC045CF51C55AD54B9A3B5F22A0` (break `/Game/Blueprints/Charater/Test/ST_ItemInfo` _output_get)) (`self.Attack`)))
      (bind _asbp_hud (cast `/Game/Blueprints/Charater/BP_HUD` (`PlayerController.GetHUD` (`GameplayStatics.GetPlayerController` 0))))
      (bind _testwidget (`/Game/Blueprints/Charater/BP_HUD.TestWidget` _asbp_hud))
      (`/Game/Blueprints/Charater/Test/WBP_TestWidget.UpdateImage` _testwidget (break `/Game/Blueprints/Charater/Test/ST_ItemInfo` _output_get))
      (`/Game/Blueprints/Charater/Test/WBP_TestWidget.UpdateText` _testwidget (`KismetTextLibrary.Conv_IntToText` (`self.HP`)) (`KismetTextLibrary.Conv_IntToText` (`self.Attack`)) (`KismetTextLibrary.Conv_IntToText` (`self.Speed`)) (`.ItemName_15_7772E27E4698011BE89391AE3DA53EBA` (break `/Game/Blueprints/Charater/Test/ST_ItemInfo` _output_get)))
      (`UserWidget.AddToViewport` (`/Game/Blueprints/Charater/BP_HUD.TestWidget` _asbp_hud) 0))))

(fn `UpdatePoseState`
  (params (NewState :type "/Game/Blueprints/Datas/Enum/E_PoseState Enum" :default "NewEnumerator0"))
  (set `self.CurrentStatePose` NewState))

(fn `UserConstructionScript`)