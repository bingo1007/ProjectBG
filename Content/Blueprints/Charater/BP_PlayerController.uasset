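; Player controller that routes movement, look, free-look, jump, crouch, prone, walk and run input to BP_Player.
; Pose keys resolve the target pose and transition time through data tables, with timed transitions disabling movement input.
; Each pose change refreshes walk speed, per-pose pitch limits and camera height, which also reacts to movement-state broadcasts.
; Timelines smoothly rotate out-of-range pitch back to the nearest limit and interpolate spring arm height.
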(event `self.ReceiveBeginPlay`
  (bind _asbp_player (cast `/Game/Blueprints/Charater/BP_Player` (`GameplayStatics.GetPlayerCharacter` 0)))
  (set `self.PlayerRef` _asbp_player)
  ; 카메라 초기화
  (`self.UpdatePitchLimits` "NewEnumerator0")
  ; 방송을 받으면 이 이벤트를 실행하겠다. 방송 = 움직임이 바뀌는 상태. 움직? 멈?
  (add `/Game/Blueprints/Charater/BP_Player.OnMovementStateChanged` (`self.PlayerRef`) (delegate `OnMovementStateChanged`))
  (`/Game/Blueprints/Charater/BP_Player.CachedWalkSpeedByPose` (`self.PlayerRef`)))

(event `OnMovementStateChanged`
  (params (bIsMoving :type Boolean))
  ; 방송을 받으면 이 이벤트를 실행하겠다. 방송 = 움직임이 바뀌는 상태. 움직? 멈?
  (`self.UpdateCameraHeight` bIsMoving))

(event `InputAxis|MoveForward`
  (params (AxisValue :type "Float (single-precision)"))
  ; 이동
  (if (`self.bIsEnableMove`)
    (`/Game/Blueprints/Charater/BP_Player.UpdateDirectionalSpeed` (`self.PlayerRef`))
    (`/Game/Blueprints/Charater/BP_Player.Move` (`self.PlayerRef`) true AxisValue)))

(event `InputAxis|MoveRight`
  (params (AxisValue :type "Float (single-precision)"))
  ; 이동
  (if (`self.bIsEnableMove`)
    (`/Game/Blueprints/Charater/BP_Player.UpdateDirectionalSpeed` (`self.PlayerRef`))
    (`/Game/Blueprints/Charater/BP_Player.Move` (`self.PlayerRef`) false AxisValue)))

(event `InputAxis|Turn`
  (params (AxisValue :type "Float (single-precision)"))
  ; 회전
  (`/Game/Blueprints/Charater/BP_Player.InputTurn` (`self.PlayerRef`) AxisValue))

(event `InputAction|PreLook`
  (params (Key :type "Key Structure"))
  (bind _playerref (`self.PlayerRef`))
  ; 프리룩
  (:`Pressed`
    (`/Game/Blueprints/Charater/BP_Player.FreeLook` _playerref true))
  (:`Released`
    (`/Game/Blueprints/Charater/BP_Player.FreeLook` _playerref false)))

(event `InputAxis|LookUp`
  (params (AxisValue :type "Float (single-precision)"))
  ; 회전
  (bind _newparam (`self.LimitPitchAngle` AxisValue))
  (if _newparam
    (`/Game/Blueprints/Charater/BP_Player.InputLookUp` (`self.PlayerRef`) AxisValue)))

(event `SetEnableMove`
  (set `self.bIsEnableMove` true))

(event `InputAction|Crouch`
  (params (Key :type "Key Structure"))
  (bind _playerref (`self.PlayerRef`))
  (bind (_transitiontype _topose) (`self.OnTransitionTimer` (`/Game/Blueprints/Charater/BP_Player.bIsWeaponEquiped` _playerref) "NewEnumerator1" (`/Game/Blueprints/Charater/BP_Player.CurrentStatePose` _playerref)))
  ; 앉음 키
  (:`Pressed`
    (`self.UpdatePose` _transitiontype _topose)))

(event `InputAction|Prone`
  (params (Key :type "Key Structure"))
  (bind _playerref (`self.PlayerRef`))
  (bind (_transitiontype _topose) (`self.OnTransitionTimer` (`/Game/Blueprints/Charater/BP_Player.bIsWeaponEquiped` _playerref) "NewEnumerator2" (`/Game/Blueprints/Charater/BP_Player.CurrentStatePose` _playerref)))
  ; 누움 키
  (:`Pressed`
    (`self.UpdatePose` _transitiontype _topose)))

(event `InputAction|Jump`
  (params (Key :type "Key Structure"))
  (bind _playerref (`self.PlayerRef`))
  (bind _currentstatepose (`/Game/Blueprints/Charater/BP_Player.CurrentStatePose` _playerref))
  (bind (_transitiontype _topose) (`self.OnTransitionTimer` (`/Game/Blueprints/Charater/BP_Player.bIsWeaponEquiped` _playerref) "NewEnumerator0" _currentstatepose))
  ; 점프 키
  (:`Pressed`
    (if (`|EnumEquality` _currentstatepose "NewEnumerator0")
      (`Character.Jump` (`self.PlayerRef`))
      (else
        (`self.UpdatePose` _transitiontype _topose)))))

(event `InputAction|Walk`
  (params (Key :type "Key Structure"))
  (bind _playerref (`self.PlayerRef`))
  ; walk 누르면 상태가 walk, 떼면 Jog
  (:`Pressed`
    (set `/Game/Blueprints/Charater/BP_Player.bIsWalkPressed` true _playerref)
    (`/Game/Blueprints/Charater/BP_Player.EvaluateMoveState` _playerref :!label _label)
    (`/Game/Blueprints/Charater/BP_Player.CachedWalkSpeedByPose` (`self.PlayerRef`)))
  (:`Released`
    (set `/Game/Blueprints/Charater/BP_Player.bIsWalkPressed` false _playerref)
    (goto _label)))

(event `InputAction|Run`
  (params (Key :type "Key Structure"))
  (bind _playerref (`self.PlayerRef`))
  ; Run, 누르면 Run, 떼면 Jog
  (:`Pressed`
    (set `/Game/Blueprints/Charater/BP_Player.bIsRunPressed` true _playerref)
    (`/Game/Blueprints/Charater/BP_Player.EvaluateMoveState` _playerref :!label _label_2)
    (`/Game/Blueprints/Charater/BP_Player.CachedWalkSpeedByPose` (`self.PlayerRef`)))
  (:`Released`
    (set `/Game/Blueprints/Charater/BP_Player.bIsRunPressed` false _playerref)
    (goto _label_2)))

(event `Set Camera Rotation`
  (bind (_direction _alpha) (`Timeline|Timeline` :!via `PlayFromStart`)
    (:`Update`
      (`self.SetControlRotation` (`KismetMathLibrary.RLerp` (`self.GetControlRotation`) (`self.EndRotation`) _alpha true)))))

(event `Set Camera Height`
  (bind (_socketoffset_x _socketoffset_y) (`KismetMathLibrary.BreakVector` (`SpringArmComponent.SocketOffset` (`/Game/Blueprints/Charater/BP_Player.SpringArm` (`self.PlayerRef`)))))
  (bind (_direction _alpha) (`Timeline|Timeline_Height` :!via `PlayFromStart`)
    (:`Update`
      (set `SpringArmComponent.SocketOffset` (`KismetMathLibrary.MakeVector` _socketoffset_x _socketoffset_y (`KismetMathLibrary.Lerp` (`self.StartHeight`) (`self.EndHeight`) _alpha)) (`/Game/Blueprints/Charater/BP_Player.SpringArm` (`self.PlayerRef`))))))

(fn `LimitPitchAngle`
  (params (Axis :type "Float (double-precision)"))
  (returns (NewParam :type Boolean))
  (bind (_returnvalue_roll _returnvalue_pitch) (`KismetMathLibrary.BreakRotator` (`self.GetControlRotation`)))
  (bind _returnvalue (+ _returnvalue_pitch (* (`local.Axis`) (`self.GetDeprecatedInputPitchScale`))))
  (return (or (> _returnvalue (`self.CachedBottomLimit`)) (< _returnvalue (`self.CachedTopLimit`)))))

(fn `OnTransitionTimer`
  (params (bIsWeaponEquiped :type Boolean) (TargetPose :type "/Game/Blueprints/Datas/Enum/Character/E_PoseState Enum" :default "NewEnumerator0") (FromPose :type "/Game/Blueprints/Datas/Enum/Character/E_PoseState Enum" :default "NewEnumerator0"))
  (returns (TransitionType :type "Float (double-precision)") (ToPose :type "/Game/Blueprints/Datas/Enum/Character/E_PoseState Enum"))
  (locals (ReturnPose :type "/Game/Blueprints/Datas/Enum/Character/E_PoseState Enum" :default "NewEnumerator0"))
  (set `local.ReturnPose` (`self.TryGetPoseTransition` TargetPose FromPose))
  (bind _returnvalue (`|GetDataTableRow` "/Game/Blueprints/Datas/DataTables/Character/DT_ProneTime.DT_ProneTime" (`KismetStringLibrary.Conv_StringToName` (`KismetStringLibrary.Concat_StrStr` (`KismetStringLibrary.Conv_BoolToString` (`local.bIsWeaponEquiped`)) "_" (`|GetEnumeratorNameAsString` (`local.FromPose`)) "_" (`|GetEnumeratorNameAsString` (`local.ReturnPose`)))))
    (:`then`
      _)
    (:`RowNotFound`
      _))
  (return (break `/Game/Blueprints/Datas/Struct/Character/ST_ProneTime` _returnvalue) (`local.ReturnPose`)))

(fn `TryGetPoseTransition`
  (params (TargetPose :type "/Game/Blueprints/Datas/Enum/Character/E_PoseState Enum" :default "NewEnumerator0") (FromPose :type "/Game/Blueprints/Datas/Enum/Character/E_PoseState Enum" :default "NewEnumerator0"))
  (returns (ToPose :type "/Game/Blueprints/Datas/Enum/Character/E_PoseState Enum"))
  (bind _returnvalue (`|GetDataTableRow` "/Game/Blueprints/Datas/DataTables/Character/DT_PoseTransitionRule.DT_PoseTransitionRule" (`KismetStringLibrary.Conv_StringToName` (`KismetStringLibrary.Concat_StrStr` (`|GetEnumeratorNameAsString` TargetPose) "_" (`|GetEnumeratorNameAsString` FromPose))))
    (:`then`
      (return (break `/Game/Blueprints/Datas/Struct/Character/ST_PoseTransitionRule` _returnvalue)))))

(fn `UpdateCameraHeight`
  (params (bIsMovingNow :type Boolean))
  (locals (CurrentPose :type String) (RowName :type String))
  (bind _currentstatepose (`/Game/Blueprints/Charater/BP_Player.CurrentStatePose` (`self.PlayerRef`)))
  (bind (_socketoffset_x _socketoffset_y _socketoffset_z) (`KismetMathLibrary.BreakVector` (`SpringArmComponent.SocketOffset` (`/Game/Blueprints/Charater/BP_Player.SpringArm` (`self.PlayerRef`)))))
  ; 자세에 따른 카메라 높이 조절
  (`|ExecutionSequence`
    (:`then_0`
      (set `local.CurrentPose` (`|GetEnumeratorNameAsString` _currentstatepose))
      (if (`|EnumInequality` _currentstatepose "NewEnumerator1")
        ;; Crouch가 아니라면 현재 상태가 곧 Row Name
        (set `local.RowName` (`local.CurrentPose`))
        (else
          (set `local.RowName` (`local.CurrentPose`))
          (if (`local.bIsMovingNow`)
            (set `local.RowName` (`KismetStringLibrary.Concat_StrStr` (`local.RowName`) "_" (`KismetStringLibrary.Conv_BoolToString` (`/Game/Blueprints/Charater/BP_Player.bIsWeaponEquiped` (`self.PlayerRef`))) "_" "Move"))))))
    (:`then_1`
      (bind _returnvalue (`|GetDataTableRow` "/Game/Blueprints/Datas/DataTables/Character/DT_CameraHeight.DT_CameraHeight" (`KismetStringLibrary.Conv_StringToName` (`local.RowName`)))
        (:`then`
          (set `self.StartHeight` _socketoffset_z)
          (set `self.EndHeight` (break `/Game/Blueprints/Datas/Struct/Character/ST_CameraHeight` _returnvalue))
          (`self.Set Camera Height`))))))

(fn `UpdatePitchLimits`
  (params (NewState :type "/Game/Blueprints/Datas/Enum/Character/E_PoseState Enum" :default "NewEnumerator0"))
  (bind (_returnvalue_roll _returnvalue_pitch _returnvalue_yaw) (`KismetMathLibrary.BreakRotator` (`self.GetControlRotation`)))
  (bind (_returnvalue_roll_2 _returnvalue_pitch_2 _returnvalue_yaw_2) (`KismetMathLibrary.BreakRotator` (`self.GetControlRotation`)))
  (bind (_returnvalue_roll_3 _returnvalue_pitch_3) (`KismetMathLibrary.BreakRotator` (`self.GetControlRotation`)))
  (`|ExecutionSequence`
    (:`then_0`
      (bind _returnvalue (`|GetDataTableRow` "/Game/Blueprints/Datas/DataTables/Character/DT_PitchLimit.DT_PitchLimit" (`KismetStringLibrary.Conv_StringToName` (`|GetEnumeratorNameAsString` (`local.NewState`))))
        (:`then`
          (set `self.CachedTopLimit` (break `/Game/Blueprints/Datas/Struct/Character/ST_PitchLimit` _returnvalue))
          (set `self.CachedBottomLimit` (`.BottomLimit_4_D24B56BB4EF7A2AFAAD0B9AEEC062E41` (break `/Game/Blueprints/Datas/Struct/Character/ST_PitchLimit` _returnvalue))))))
    (:`then_1`
      ; 현재 카메라 각도가 limit 각도를 초과했는지 확인
      (if (not (or (> _returnvalue_pitch_3 (`self.CachedBottomLimit`)) (< _returnvalue_pitch_3 (`self.CachedTopLimit`))))
        (if (< (`KismetMathLibrary.Abs` (- _returnvalue_pitch_3 (`self.CachedTopLimit`))) (`KismetMathLibrary.Abs` (- _returnvalue_pitch_3 (`self.CachedBottomLimit`))))
          (set `self.EndRotation` (`KismetMathLibrary.MakeRotator` _returnvalue_roll_2 (`self.CachedTopLimit`) _returnvalue_yaw_2))
          (else
            (set `self.EndRotation` (`KismetMathLibrary.MakeRotator` _returnvalue_roll (`self.CachedBottomLimit`) _returnvalue_yaw))))
        (`self.Set Camera Rotation`)))))

(fn `UpdatePose`
  (params (WaitTime :type "Float (double-precision)") (ToPose :type "/Game/Blueprints/Datas/Enum/Character/E_PoseState Enum" :default "NewEnumerator0"))
  (`|ExecutionSequence`
    (:`then_0`
      (if (!= WaitTime 0.0)
        (set `self.bIsEnableMove` false)
        (`KismetSystemLibrary.K2_SetTimerDelegate` (`|CreateDelegate` :!event `SetEnableMove`) (`local.WaitTime`))
        (`/Game/Blueprints/Charater/BP_Player.UpdatePoseState` (`self.PlayerRef`) (`local.ToPose`))
        (else
          (`/Game/Blueprints/Charater/BP_Player.UpdatePoseState` (`self.PlayerRef`) (`local.ToPose`)))))
    (:`then_1`
      (`self.UpdatePitchLimits` (`local.ToPose`))
      (`self.UpdateCameraHeight` (`/Game/Blueprints/Charater/BP_Player.bIsMovingNow` (`self.PlayerRef`)))
      (`/Game/Blueprints/Charater/BP_Player.CachedWalkSpeedByPose` (`self.PlayerRef`)))))

(fn `UserConstructionScript`)