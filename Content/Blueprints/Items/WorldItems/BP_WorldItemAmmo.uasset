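; BP_WorldItemAmmo is a world item for an ammo pickup that represents a bundle of rounds.
; InitSpawnData looks up its row in DT_WorldItem_AmmoData by ID, initializes the shared world item base data, and stores the pickup amount and per-unit weight.
; GetWeight returns the bundle's total weight as amount times single weight.
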(fn `GetWeight`
  (returns (Weight :type Integer))
  ; single weight와 곱해서 실제 묶음의 무게 계산
  (return (* (`self.Amount`) (`self.SingleWeight`))))

(fn `InitSpawnData`
  (params (ID :type Name) (SN :type String))
  (`parent.InitSpawnData` ID SN)
  (bind _returnvalue (`|GetDataTableRow` "/Game/Blueprints/Datas/DataTables/Item/DT_WorldItem_AmmoData.DT_WorldItem_AmmoData" (`self.ID`))
    (:`then`
      (`self.InitWorldItemBaseData` (break `/Game/Blueprints/Datas/Struct/Item/ST_WorldItem_AmmoData` _returnvalue) (`.ItemName_5_43371B42480220238AC49DABB62CE6BE` (break `/Game/Blueprints/Datas/Struct/Item/ST_WorldItem_AmmoData` _returnvalue)) (`.UiPreFix_8_DE9894C140AE2B69798C19BD8A93F7E6` (break `/Game/Blueprints/Datas/Struct/Item/ST_WorldItem_AmmoData` _returnvalue)) (`.StaticMesh_11_7F1D3C234D3E871163055F86A6AB613B` (break `/Game/Blueprints/Datas/Struct/Item/ST_WorldItem_AmmoData` _returnvalue)))
      (set `self.Amount` (`.PickUpAmmo_14_1ECF6792434BCEE128C460892DE8841A` (break `/Game/Blueprints/Datas/Struct/Item/ST_WorldItem_AmmoData` _returnvalue)))
      (set `self.SingleWeight` (`.Weight_16_46C87DA446CD25063E9461BD2A8F1C74` (break `/Game/Blueprints/Datas/Struct/Item/ST_WorldItem_AmmoData` _returnvalue))))))

(fn `UserConstructionScript`
  (`parent.UserConstructionScript`))