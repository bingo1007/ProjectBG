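; World item Blueprint for weapon accessories: sights, muzzles, foregrips, magazines and buttstocks.
; InitSpawnData looks up the spawn ID in DT_WorldItem_AccData and passes type, name, UI prefix and mesh to InitWorldItemBaseData.
; It also stores accessory type and weight, then corrects placement with the row's world rotation offset.
; Every type except Sight is raised by its mesh bounds' Z half-extent.
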(fn `InitSpawnData`
  (params (ID :type Name) (SN :type String))
  (bind (_origin _boxextent) (`KismetSystemLibrary.GetComponentBounds` (`self.StaticMesh`)))
  (`parent.InitSpawnData` ID SN)
  (bind _returnvalue (`|GetDataTableRow` "/Game/Blueprints/Datas/DataTables/Item/DT_WorldItem_AccData.DT_WorldItem_AccData" (`self.ID`))
    (:`then`
      (`self.InitWorldItemBaseData` (break `/Game/Blueprints/Datas/Struct/Item/ST_WorldItem_AccData` _returnvalue) (`.ItemName_5_87A80A76480FA3C01A40E6BBF4844188` (break `/Game/Blueprints/Datas/Struct/Item/ST_WorldItem_AccData` _returnvalue)) (`.UiPreFix_8_B2F61DCC44D5B8D6BF60DF81871A03AA` (break `/Game/Blueprints/Datas/Struct/Item/ST_WorldItem_AccData` _returnvalue)) (`.StaticMesh_14_971286E244ACAF2719CAA9B89BAC9D82` (break `/Game/Blueprints/Datas/Struct/Item/ST_WorldItem_AccData` _returnvalue)))
      (set `self.AccType` (`.Type_11_F4B0F9854FC4786AD2503FAF66D9CBE6` (break `/Game/Blueprints/Datas/Struct/Item/ST_WorldItem_AccData` _returnvalue)))
      (set `self.Out Row Weight` (`.Weight_20_0A0BDF0B49D755F7CA64DFB127F8C60E` (break `/Game/Blueprints/Datas/Struct/Item/ST_WorldItem_AccData` _returnvalue)))
      ; 회전 보정
      (`SceneComponent.K2_SetWorldRotation` (`self.StaticMesh`) (`.RotationOffset_21_934CBF724989AB4C976BEDBEB2D665C2` (break `/Game/Blueprints/Datas/Struct/Item/ST_WorldItem_AccData` _returnvalue)) false false)
      (`self.K2_AddActorLocalOffset` (`KismetMathLibrary.MakeVector` 0.0 0.0 (select `/Game/Blueprints/Datas/Enum/Item/E_WeaponAcceseryType` (`self.AccType`) :`NewEnumerator1` (.z _boxextent) :`NewEnumerator2` (.z _boxextent) :`NewEnumerator3` (.z _boxextent) :`NewEnumerator4` (.z _boxextent)))))))

(fn `UserConstructionScript`
  (`parent.UserConstructionScript`))