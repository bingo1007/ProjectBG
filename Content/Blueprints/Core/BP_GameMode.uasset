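; Game mode that, on BeginPlay, spawns item groups and rolls a random set of item types.
; GenerateItems spawns a BP_ItemGroup at every DT_ItemGroupLocation row, then makes one count roll and adds that many rolled types to ItemTypeArray.
; Count and type rolls are weighted by repeating each probability-table value Percent times in an array and picking randomly.
; The rolled types are not passed to the spawned groups here.
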(event `self.ReceiveBeginPlay`
  (`self.GenerateItems`))

(fn `GenerateItems`
  (locals (ItemTypeArray :type "Array of /Game/Blueprints/Datas/Enum/ItemGeneration/E_ItemType Enum"))
  ; 8개의 아이템 그룹에 대해 랜덤한 위치와 아이템 타입 + 아이템 개수 생성
  (`|ExecutionSequence`
    (:`then_0`
      (bind _outrownames (`DataTableFunctionLibrary.GetDataTableRowNames` "/Game/Blueprints/Datas/DataTables/ItemGeneration/DT_ItemGroupLocation.DT_ItemGroupLocation"))
      (for _array_element _outrownames
        (bind _returnvalue (`|GetDataTableRow` "/Game/Blueprints/Datas/DataTables/ItemGeneration/DT_ItemGroupLocation.DT_ItemGroupLocation" _array_element)
          (:`then`
            (`|SpawnActorFromClass` "/Game/Blueprints/Items/BP_ItemGroup.BP_ItemGroup_C" (`KismetMathLibrary.MakeTransform` (break `/Game/Blueprints/Datas/Struct/ItemGeneration/ST_ItemGroupLocation` _returnvalue)) "AlwaysSpawn" "MultiplyWithRoot" null null)))))
    (:`then_1`
      (bind _number (`self.RandomItemNumber`))
      (for _ (range 1 (+ _number 1))
        (bind _newparam (`self.RandomItemType`))
        (`KismetArrayLibrary.Array_Add` (`local.ItemTypeArray`) _newparam)))))

(fn `RandomItemNumber`
  (returns (Number :type Integer))
  (locals (NumberArr :type "Array of Integer"))
  (bind _outrownames (`DataTableFunctionLibrary.GetDataTableRowNames` "/Game/Blueprints/Datas/DataTables/ItemGeneration/DT_NumberProbability.DT_NumberProbability"))
  (for _array_element _outrownames
    (bind _returnvalue (`|GetDataTableRow` "/Game/Blueprints/Datas/DataTables/ItemGeneration/DT_NumberProbability.DT_NumberProbability" _array_element)
      (:`then`
        (for _ (range 1 (+ (break `/Game/Blueprints/Datas/Struct/ItemGeneration/ST_NumberProbability` _returnvalue) 1))
          (`KismetArrayLibrary.Array_Add` (`local.NumberArr`) (`.Number_5_DBA6A6D348572398CB2E3C843A22E6F9` (break `/Game/Blueprints/Datas/Struct/ItemGeneration/ST_NumberProbability` _returnvalue)))))))
  (return (`KismetArrayLibrary.Array_Random` (`local.NumberArr`))))

(fn `RandomItemType`
  (returns (NewParam :type "/Game/Blueprints/Datas/Enum/ItemGeneration/E_ItemType Enum"))
  (locals (ItemTypeArray :type "Array of /Game/Blueprints/Datas/Enum/ItemGeneration/E_ItemType Enum"))
  (bind _outrownames (`DataTableFunctionLibrary.GetDataTableRowNames` "/Game/Blueprints/Datas/DataTables/ItemGeneration/DT_ItemTypeProbability.DT_ItemTypeProbability"))
  (for _array_element _outrownames
    (bind _returnvalue (`|GetDataTableRow` "/Game/Blueprints/Datas/DataTables/ItemGeneration/DT_ItemTypeProbability.DT_ItemTypeProbability" _array_element)
      (:`then`
        (for _ (range 1 (+ (break `/Game/Blueprints/Datas/Struct/ItemGeneration/ST_ItemTypeProbability` _returnvalue) 1))
          (`KismetArrayLibrary.Array_Add` (`local.ItemTypeArray`) (`.ItemType_10_0336C3524A8FBADC038809906BD84AC5` (break `/Game/Blueprints/Datas/Struct/ItemGeneration/ST_ItemTypeProbability` _returnvalue)))))))
  (return (`KismetArrayLibrary.Array_Random` (`local.ItemTypeArray`))))

(fn `UserConstructionScript`)